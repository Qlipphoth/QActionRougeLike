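; Red barrel actor that explodes on a server-started timer shortly after BeginPlay.
; The authority-only timer calls Explode, which triggers MulticastExplode to print a debug string, fire the radial force impulse and disable collision.
; SetActorHiddenInGame is passed false, so the explosion does not hide the barrel.
; A short lifespan removes the actor afterwards, because destroying it immediately would invalidate the multicast.
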(event `self.ReceiveBeginPlay`
  (`/Engine/EditorBlueprintResources/ActorMacros.Switch Has Authority`
    (:`Authority`
      (`KismetSystemLibrary.K2_SetTimerDelegate` (delegate `Explode`) 4.0))))

(event `Explode`
  (`self.MulticastExplode`)
  (`self.SetLifeSpan` 2.0))

(event `MulticastExplode`
  (`KismetSystemLibrary.PrintString` "Explode")
  (`RadialForceComponent.FireImpulse` (`self.RadialForceComp`))
  (`self.SetActorHiddenInGame` false)
  (`self.SetActorEnableCollision` false))

(fn `UserConstructionScript`)